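; Mario2 is an actor Blueprint that moves left and right along the world X axis from keyboard input.
; The A and D keys set a Direction variable to negative or positive while held and clear it on release.
; Tick offsets the actor's location by Direction times a fixed step each frame, without sweep or delta-time scaling, so movement ignores collision and depends on frame rate.
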(event `Key|SpaceBar`
  (params (Key :type "Key Structure")))

(event `Key|A`
  (params (Key :type "Key Structure"))
  (:`Pressed`
    (set `self.direction` -1.0))
  (:`Released`
    (set `self.direction` 0.0)))

(event `Key|D`
  (params (Key :type "Key Structure"))
  (:`Pressed`
    (set `self.direction` 1.0))
  (:`Released`
    (set `self.direction` 0.0)))

(event `self.ReceiveTick`
  (params (DeltaSeconds :type "Float (single-precision)"))
  (`self.K2_SetActorLocation` (+ (`self.K2_GetActorLocation`) (`KismetMathLibrary.MakeVector` (* (`self.direction`) 3.0)))))

(fn `UserConstructionScript`)